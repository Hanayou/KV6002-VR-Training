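; Player character with axis-driven movement and look controls, linked to the safety game mode for objective recording.
; Movement follows control-rotation yaw only, while Turn and LookUp feed controller yaw and pitch.
; Escape/Back shows the mouse cursor with game-and-UI input, and a left click restores game-only focus.
; The game mode is cached on BeginPlay so a debug input can record a randomly passed or failed test objective.
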(event EventBeginPlay
  (bind _asbp_safety_game_mode (Utilities|Casting|CastToBP_SafetyGameMode (Game|GetGameMode)))
  (Variables|Default|SetAs%20BP%20Safety%20Game%20Mode _asbp_safety_game_mode))

(event Input|ActionEvents|InputActionEscape/Back
  (params (Key :type Key%20Structure :default "None"))
  (bind _returnvalue (Game|GetPlayerController 0))
  ;[1 1 1] Press Esc in-game to show mouse cursor / click to re-focus game
  (:Pressed
    (Development|PrintString "Escape/Back Event Called!")
    (Input|SetInputModeGameandUI _returnvalue 0 "DoNotLock" false false)
    (Variables|/Script/Engine.PlayerController|SetbShowMouseCursor _returnvalue true)))

(event Input|ActionEvents|InputActionDEBUG_ForceAddObjective
  (params (Key :type Key%20Structure :default "None"))
  (bind _as_bp_safety_game_mode (Variables|Default|GetAs%20BP%20Safety%20Game%20Mode))
  ;[1 1 1] DEBUG: Force objective to be triggered
  (:Pressed
    (if (Math|Random|RandomBoolfromStream (Math|Random|MakeRandomStream (Math|Random|RandomInteger 10000)))
      (Default|RecordObjective _as_bp_safety_game_mode true "This is a succesful debug objective, not for use in production gameplay!" 250)
      (else
        (Default|RecordObjective _as_bp_safety_game_mode false "This is a failed debug objective, not for use in production gameplay!")))))

(event Input|AxisEvents|InputAxisMoveForward
  (params (AxisValue :type Float%20%28single-precision%29))
  ;[1 1 1] Directional Movement
  (Pawn|Input|AddMovementInput (Math|Vector|GetForwardVector (Math|Rotator|MakeRotator 0.0 0.0 (.Yaw (Math|Rotator|BreakRotator (Pawn|GetControlRotation :!class /Script/Engine.Pawn))))) AxisValue false))

(event Input|AxisEvents|InputAxisMoveRight
  (params (AxisValue :type Float%20%28single-precision%29))
  ;[1 1 1] Directional Movement
  (Pawn|Input|AddMovementInput (Math|Vector|GetRightVector (Math|Rotator|MakeRotator 0.0 0.0 (.Yaw (Math|Rotator|BreakRotator (Pawn|GetControlRotation :!class /Script/Engine.Pawn))))) AxisValue false))

(event Input|AxisEvents|InputAxisLookUp
  (params (AxisValue :type Float%20%28single-precision%29))
  ;[1 1 1] View Rotation Input
  (Pawn|Input|AddControllerPitchInput AxisValue))

(event Input|AxisEvents|InputAxisTurn
  (params (AxisValue :type Float%20%28single-precision%29))
  ;[1 1 1] View Rotation Input
  (Pawn|Input|AddControllerYawInput AxisValue))

(event Input|MouseEvents|LeftMouseButton
  (params (Key :type Key%20Structure :default "None"))
  (bind _returnvalue (Game|GetPlayerController 0))
  ;[1 1 1] Press Esc in-game to show mouse cursor / click to re-focus game
  (:Pressed
    (Class|WidgetBlueprintLibrary|SetFocustoGameViewport)
    (Input|SetInputModeGameOnly _returnvalue false)
    (Variables|/Script/Engine.PlayerController|SetbShowMouseCursor _returnvalue false)))

(fn ConstructionScript)