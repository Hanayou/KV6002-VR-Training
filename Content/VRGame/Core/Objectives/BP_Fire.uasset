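; BP_Fire is an interactable fire hazard objective in the VR safety game that the player puts out with a fire extinguisher.
; Overlapping its box shows an interact prompt and sets a flag checked when the player's bound interact key fires.
; If the player's extinguisher is visible, it reveals the player's steam effect and records a successful objective with points in BP_SafetyGameMode.
; After a short delay it hides the extinguisher and destroys itself.
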(event OnComponentBeginOverlap(Box)
  (params (OverlappedComponent :type Primitive%20Component%20Object%20Reference) (OtherActor :type Actor%20Object%20Reference) (OtherComp :type Primitive%20Component%20Object%20Reference) (OtherBodyIndex :type Integer) (bFromSweep :type Boolean) (SweepResult :type Hit%20Result%20Structure%20%28by%20ref%29))
  (Utilities|Casting|CastToBP_PlayerCharacter OtherActor)
  (Variables|Default|SetbIsOverlappingBox true)
  (Default|ShowInteractUI (Variables|Default|GetInteractionUIComonent)))

(event OnComponentEndOverlap(Box)
  (params (OverlappedComponent :type Primitive%20Component%20Object%20Reference) (OtherActor :type Actor%20Object%20Reference) (OtherComp :type Primitive%20Component%20Object%20Reference) (OtherBodyIndex :type Integer))
  (Utilities|Casting|CastToBP_PlayerCharacter OtherActor)
  (Variables|Default|SetbIsOverlappingBox false)
  (Default|HideInteractUI (Variables|Default|GetInteractionUIComonent)))

(event Custom|InteractKeyPressed
  (bind _asbp_player_character (Utilities|Casting|CastToBP_PlayerCharacter (Game|GetPlayerCharacter 0)))
  (if (and (Variables|Default|GetbIsOverlappingBox) (not (Variables|/Script/Engine.SceneComponent|GetbHiddenInGame (Variables|/Game/VRGame/Characters/BP_PlayerCharacter.BP_PlayerCharacter_C|GetFireExtinguisher _asbp_player_character))))
    (Development|SetHiddeninGame (Variables|/Game/VRGame/Characters/BP_PlayerCharacter.BP_PlayerCharacter_C|GetSteam _asbp_player_character) false false)
    (bind _asbp_safety_game_mode (Utilities|Casting|CastToBP_SafetyGameMode (Game|GetGameMode)))
    (Default|RecordObjective _asbp_safety_game_mode true "Fire extinquished! The break room is saved!" 250)
    (bind _asbp_player_character_2 (Utilities|Casting|CastToBP_PlayerCharacter (Game|GetPlayerCharacter 0)))
    (Utilities|FlowControl|Delay 1.0)
    (Development|SetHiddeninGame (Variables|/Game/VRGame/Characters/BP_PlayerCharacter.BP_PlayerCharacter_C|GetFireExtinguisher _asbp_player_character_2) true true)
    (Actor|DestroyActor)))

(event EventBeginPlay
  (bind _asbp_player_character (Utilities|Casting|CastToBP_PlayerCharacter (Game|GetPlayerCharacter 0)))
  (EventDispatchers|BindEventtoInteractKeyPressed _asbp_player_character (delegate Custom|InteractKeyPressed)))

(fn ConstructionScript)