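; BP_FluidSpillage is a cleanable spill objective in the safety game that slows the player while they stand in it.
; Box overlap toggles the interact prompt and drops the player's walk speed, restoring it on exit.
; The player's interact key, bound at BeginPlay, records a scored success with BP_SafetyGameMode if they overlap it with the mop visible.
; After a short delay, it hides the mop and destroys itself.
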(event OnComponentBeginOverlap(Box)
  (params (OverlappedComponent :type Primitive%20Component%20Object%20Reference) (OtherActor :type Actor%20Object%20Reference) (OtherComp :type Primitive%20Component%20Object%20Reference) (OtherBodyIndex :type Integer) (bFromSweep :type Boolean) (SweepResult :type Hit%20Result%20Structure%20%28by%20ref%29))
  (bind _asbp_player_character (Utilities|Casting|CastToBP_PlayerCharacter OtherActor))
  (Variables|Default|SetbIsOverlapping true)
  (Default|ShowInteractUI (Variables|Default|GetInteractionUIComonent))
  (bind _ascharacter_movement_component (Utilities|Casting|CastToCharacterMovementComponent (Pawn|GetMovementComponent _asbp_player_character)))
  (Variables|/Script/Engine.CharacterMovementComponent|SetMaxWalkSpeed _ascharacter_movement_component 2e+02))

(event OnComponentEndOverlap(Box)
  (params (OverlappedComponent :type Primitive%20Component%20Object%20Reference) (OtherActor :type Actor%20Object%20Reference) (OtherComp :type Primitive%20Component%20Object%20Reference) (OtherBodyIndex :type Integer))
  (bind _asbp_player_character (Utilities|Casting|CastToBP_PlayerCharacter OtherActor))
  (Variables|Default|SetbIsOverlapping false)
  (Default|HideInteractUI (Variables|Default|GetInteractionUIComonent))
  (bind _ascharacter_movement_component (Utilities|Casting|CastToCharacterMovementComponent (Pawn|GetMovementComponent _asbp_player_character)))
  (Variables|/Script/Engine.CharacterMovementComponent|SetMaxWalkSpeed _ascharacter_movement_component 6e+02))

(event Custom|InteractKeyPressed
  (bind _asbp_player_character (Utilities|Casting|CastToBP_PlayerCharacter (Game|GetPlayerCharacter 0)))
  (if (and (Variables|Default|GetbIsOverlapping) (not (Variables|/Script/Engine.SceneComponent|GetbHiddenInGame (Variables|/Game/VRGame/Characters/BP_PlayerCharacter.BP_PlayerCharacter_C|GetMop _asbp_player_character))))
    (bind _asbp_safety_game_mode (Utilities|Casting|CastToBP_SafetyGameMode (Game|GetGameMode)))
    (Default|RecordObjective _asbp_safety_game_mode true "I'm not sure what that fluid was, but it's all clean now!" 250)
    (bind _asbp_player_character_2 (Utilities|Casting|CastToBP_PlayerCharacter (Game|GetPlayerCharacter 0)))
    (Utilities|FlowControl|Delay 1.0)
    (Development|SetHiddeninGame (Variables|/Game/VRGame/Characters/BP_PlayerCharacter.BP_PlayerCharacter_C|GetMop _asbp_player_character_2) true false)
    (Actor|DestroyActor)))

(event EventBeginPlay
  (bind _asbp_player_character (Utilities|Casting|CastToBP_PlayerCharacter (Game|GetPlayerCharacter 0)))
  (EventDispatchers|BindEventtoInteractKeyPressed _asbp_player_character (delegate Custom|InteractKeyPressed)))

(fn ConstructionScript)