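; BP_Pipe is a repairable pipe objective for the VR game's safety game mode.
; It binds to the player character's interact key event and shows or hides an interact prompt as the player enters or leaves its box.
; Interacting while overlapping records a successful, point-awarding objective with the game mode, then destroys the box and particle system components.
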(event OnComponentBeginOverlap(Box)
  (params (OverlappedComponent :type Primitive%20Component%20Object%20Reference) (OtherActor :type Actor%20Object%20Reference) (OtherComp :type Primitive%20Component%20Object%20Reference) (OtherBodyIndex :type Integer) (bFromSweep :type Boolean) (SweepResult :type Hit%20Result%20Structure%20%28by%20ref%29))
  (Utilities|Casting|CastToBP_PlayerCharacter OtherActor)
  (Variables|Default|SetbIsOverlapping true)
  (Default|ShowInteractUI (Variables|Default|GetInteractionUIComonent)))

(event OnComponentEndOverlap(Box)
  (params (OverlappedComponent :type Primitive%20Component%20Object%20Reference) (OtherActor :type Actor%20Object%20Reference) (OtherComp :type Primitive%20Component%20Object%20Reference) (OtherBodyIndex :type Integer))
  (Utilities|Casting|CastToBP_PlayerCharacter OtherActor)
  (Variables|Default|SetbIsOverlapping false)
  (Default|HideInteractUI (Variables|Default|GetInteractionUIComonent)))

(event Custom|InteractKeyPressed
  (if (Variables|Default|GetbIsOverlapping)
    (bind _asbp_safety_game_mode (Utilities|Casting|CastToBP_SafetyGameMode (Game|GetGameMode)))
    (Default|RecordObjective _asbp_safety_game_mode true "Pipe repaired!" 250)
    (Components|DestroyComponent (Variables|Default|GetBox))
    (Components|DestroyComponent (Variables|Default|GetParticleSystem))))

(event EventBeginPlay
  (bind _asbp_player_character (Utilities|Casting|CastToBP_PlayerCharacter (Game|GetPlayerCharacter 0)))
  (EventDispatchers|BindEventtoInteractKeyPressed _asbp_player_character (delegate Custom|InteractKeyPressed)))

(fn ConstructionScript)